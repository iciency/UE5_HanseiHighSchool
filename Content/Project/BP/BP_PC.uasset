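; BP_PC is a player controller Blueprint that toggles between the player's default pawn and a free spectator camera.
; It stores the controlled pawn at BeginPlay, and a FlipFlop on the IA_SpecterMode input alternates the two states.
; Entering spawns and possesses a SpectatorPawn at that pawn's transform, hiding the pawn with tick enabled.
; Leaving destroys the spectator and repossesses the unhidden pawn, with tick disabled.
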(event Input|EnhancedActionEvents|EnhancedInputActionIA_SpecterMode
  (params (ActionValue :type Float%20%28double-precision%29) (ElapsedSeconds :type Float%20%28double-precision%29) (TriggeredSeconds :type Float%20%28double-precision%29) (InputAction :type Input%20Action%20Object%20Reference :default "/Game/ThirdPerson/Input/Actions/IA_SpecterMode.IA_SpecterMode"))
  (bind _defaultpawn (Variables|Default|GetDefaultPawn))
  (bind _defaultpawn_2 (Variables|Default|GetDefaultPawn))
  (:Started
    (Utilities|FlowControl|FlipFlop
      (:A
        (bind _returnvalue (Game|SpawnActorfromClass "/Script/Engine.SpectatorPawn" (Transformation|GetActorTransform (Variables|Default|GetDefaultPawn)) "Undefined" "MultiplyWithRoot" 0 0))
        (Variables|Default|SetSpawnSpactater _returnvalue)
        (Actor|Tick|SetActorTickEnabled _defaultpawn true)
        (Rendering|SetActorHiddenInGame _defaultpawn true)
        (Pawn|Possess (Variables|Default|GetSpawnSpactater)))
      (:B
        (Actor|DestroyActor (Variables|Default|GetSpawnSpactater))
        (Actor|Tick|SetActorTickEnabled _defaultpawn_2)
        (Rendering|SetActorHiddenInGame _defaultpawn_2 false)
        (Pawn|Possess (Variables|Default|GetDefaultPawn))))))

(event EventBeginPlay
  (Variables|Default|SetDefaultPawn (Pawn|GetControlledPawn)))

(event EventTick
  (params (DeltaSeconds :type Float%20%28single-precision%29)))

(fn ConstructionScript)