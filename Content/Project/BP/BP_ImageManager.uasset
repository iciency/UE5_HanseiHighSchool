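; BP_ImageManager manages screenshot images and reference camera transforms, apparently for a photo-matching mechanic.
; On BeginPlay it creates the screenshot list widget and parses AnswerTexture2D display names into transforms, using "l"/"_" delimiters and "e" as decimal point.
; LoadScreenshotPNGs imports screenshot-folder PNGs as textures when their count differs from the widget's, then has it spawn images.
; Trn only prints whether a captured transform is within location, pitch and yaw tolerance.
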(event Custom|LoadScreenshotPNGs
  (bind _returnvalue (Class|CaptureFunctionLibrary|GetPNGsOfPath (Class|BlueprintPathsLibrary|ScreenShotDir) "*.png"))
  (bind _output_get (Variables|Default|SetPNGsPath _returnvalue))
  (bind _output_get_2 (Variables|Default|SetPNGCount (Utilities|Array|Length _output_get)))
  (if (!= _output_get_2 (Class|PanelWidget|GetChildrenCount (Variables|/Game/Project/BP/Widget/BP_ScreenShotList.BP_ScreenShotList_C|GetWrapBox_73 (Variables|Default|GetWidget))))
    (for _array_element (Variables|Default|GetPNGsPath)
      (bind _returnvalue_2 (Class|KismetRenderingLibrary|ImportFileasTexture2D (Utilities|String|Append (Class|BlueprintPathsLibrary|ScreenShotDir) _array_element)))
      (Utilities|Array|Add (Variables|Default|GetPNGsPath%20Import%20Texture2D) _returnvalue_2))
    (Utilities|Array|Reverse (Variables|Default|GetPNGsPath%20Import%20Texture2D))
    (Utilities|Array|Clear (Variables|Default|GetPNGsPath))
    (Default|CallSpawnScreenShotImg (Variables|Default|GetWidget))))

(event Custom|pasTranfromString
  (params (TranfromString :type String))
  ;[1 1 1] 파써
  (for _array_element (Utilities|String|ParseIntoArray TranfromString "l")
    (switch string (Utilities|Array|Get(acopy) (Utilities|String|ParseIntoArray _array_element "_"))
      (:x
        (Variables|Default|SetMakeTransfrom (Math|Transform|MakeTransform (Math|Vector|MakeVector (Math|Conversions|ToFloat(Integer) (Utilities|String|Replace (Utilities|Array|Get(acopy) (Utilities|String|ParseIntoArray _array_element "_") 1) "e" ".")) (.y (.location (Variables|Default|GetMakeTransfrom))) (.z (.location (Variables|Default|GetMakeTransfrom)))) (.rotation (Variables|Default|GetMakeTransfrom)) (.scale (Variables|Default|GetMakeTransfrom)))))
      (:y
        (Variables|Default|SetMakeTransfrom (Math|Transform|MakeTransform (Math|Vector|MakeVector (.x (.location (Variables|Default|GetMakeTransfrom))) (Math|Conversions|ToFloat(Integer) (Utilities|String|Replace (Utilities|Array|Get(acopy) (Utilities|String|ParseIntoArray _array_element "_") 1) "e" ".")) (.z (.location (Variables|Default|GetMakeTransfrom)))) (.rotation (Variables|Default|GetMakeTransfrom)) (.scale (Variables|Default|GetMakeTransfrom)))))
      (:z
        (Variables|Default|SetMakeTransfrom (Math|Transform|MakeTransform (Math|Vector|MakeVector (.x (.location (Variables|Default|GetMakeTransfrom))) (.y (.location (Variables|Default|GetMakeTransfrom))) (Math|Conversions|ToFloat(Integer) (Utilities|String|Replace (Utilities|Array|Get(acopy) (Utilities|String|ParseIntoArray _array_element "_") 1) "e" "."))) (.rotation (Variables|Default|GetMakeTransfrom)) (.scale (Variables|Default|GetMakeTransfrom)))))
      (:P
        (Variables|Default|SetMakeTransfrom (Math|Transform|MakeTransform (.location (Variables|Default|GetMakeTransfrom)) (Math|Rotator|MakeRotator (.roll (.rotation (Variables|Default|GetMakeTransfrom))) (Math|Conversions|ToFloat(Integer) (Utilities|String|Replace (Utilities|Array|Get(acopy) (Utilities|String|ParseIntoArray _array_element "_") 1) "e" ".")) (.yaw (.rotation (Variables|Default|GetMakeTransfrom)))) (.scale (Variables|Default|GetMakeTransfrom)))))
      (:Y
        (Variables|Default|SetMakeTransfrom (Math|Transform|MakeTransform (.location (Variables|Default|GetMakeTransfrom)) (Math|Rotator|MakeRotator (.roll (.rotation (Variables|Default|GetMakeTransfrom))) (.pitch (.rotation (Variables|Default|GetMakeTransfrom))) (Math|Conversions|ToFloat(Integer) (Utilities|String|Replace (Utilities|Array|Get(acopy) (Utilities|String|ParseIntoArray _array_element "_") 1) "e" "."))) (.scale (Variables|Default|GetMakeTransfrom)))))))
  (Utilities|Map|Add (Variables|Default|GetScreenShotTransfrom) (Variables|Default|GetMakeTransfrom) false)
  (Variables|Default|SetMakeTransfrom ""))

(event EventBeginPlay
  (bind _answertexture2d (Variables|Default|GetAnswerTexture2D))
  (bind _returnvalue (UserInterface|CreateWidget "/Game/Project/BP/Widget/BP_ScreenShotList.BP_ScreenShotList_C"))
  (Variables|Default|SetWidget _returnvalue)
  (Utilities|Array|Reverse _answertexture2d)
  (for _array_element _answertexture2d
    (CallFunction|PasTranfromString (Utilities|GetDisplayName _array_element))))

(event EventTick
  (params (DeltaSeconds :type Float%20%28single-precision%29)))

(fn ConstructionScript)

(fn Trn
  (params (Transfrom :type Transform) (CaptureTrn :type Transform) (amount :type Float%20%28double-precision%29))
  (bind (_location _rotation) (Math|Transform|BreakTransform CaptureTrn))
  (bind _returnvalue (Math|Rotator|Delta(Rotator) _rotation (.rotation Transfrom)))
  (bind (_roll _pitch _yaw) (Math|Rotator|BreakRotator _returnvalue))
  (Development|PrintString (Utilities|String|ToString(Boolean) (Math|Boolean|ANDBoolean (>= (* amount 8.0) (Math|Float|Absolute(Float) (Math|Vector|Distance(Vector) _location (.location Transfrom)))) (>= amount (Math|Float|Absolute(Float) _pitch)) (>= amount (Math|Float|Absolute(Float) _yaw)))))
  (return "false"))