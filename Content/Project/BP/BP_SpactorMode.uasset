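; BP_SpactorMode toggles a spectator mode for the PlayerController that owns it.
; On BeginPlay it caches that controller and its controlled pawn.
; The IA_SpecterMode input drives a FlipFlop that spawns a spectator pawn at the camera's transform, possesses it and hides the original pawn.
; The next press destroys the spectator, then unhides and repossesses the original; pawn tick is enabled while spectating and disabled on return.
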(event Input|EnhancedActionEvents|EnhancedInputActionIA_SpecterMode
  (params (ActionValue :type Float%20%28double-precision%29) (ElapsedSeconds :type Float%20%28double-precision%29) (TriggeredSeconds :type Float%20%28double-precision%29) (InputAction :type Input%20Action%20Object%20Reference :default "/Game/ThirdPerson/Input/Actions/IA_SpecterMode.IA_SpecterMode"))
  (bind _defaultpawn (Variables|Default|GetDefaultPawn))
  (bind _as플레이어_컨트롤러 (Variables|Default|GetAs플레이어%20컨트롤러))
  (bind _defaultpawn_2 (Variables|Default|GetDefaultPawn))
  (bind _playercameramanager (Variables|/Script/Engine.PlayerController|GetPlayerCameraManager _as플레이어_컨트롤러))
  (:Started
    (Utilities|FlowControl|FlipFlop
      (:A
        (bind _returnvalue (Game|SpawnActorfromClass "/Script/Engine.SpectatorPawn" (Math|Transform|MakeTransform (Camera|GetCameraLocation _playercameramanager) (Camera|GetCameraRotation _playercameramanager)) "Undefined" "MultiplyWithRoot" 0 0))
        (Variables|Default|SetSpawnSpactater _returnvalue)
        (Actor|Tick|SetActorTickEnabled _defaultpawn true)
        (Rendering|SetActorHiddenInGame _defaultpawn true)
        (Pawn|Possess (Variables|Default|GetAs플레이어%20컨트롤러) (Variables|Default|GetSpawnSpactater)))
      (:B
        (Actor|DestroyActor (Variables|Default|GetSpawnSpactater))
        (Actor|Tick|SetActorTickEnabled _defaultpawn_2)
        (Rendering|SetActorHiddenInGame _defaultpawn_2 false)
        (Pawn|Possess (Variables|Default|GetAs플레이어%20컨트롤러) (Variables|Default|GetDefaultPawn))))))

(event EventBeginPlay
  (bind _as플레이어_컨트롤러 (Utilities|Casting|CastToPlayerController (Components|GetOwner)))
  (Variables|Default|SetDefaultPawn (Pawn|GetControlledPawn _as플레이어_컨트롤러))
  (bind _as플레이어_컨트롤러_2 (Utilities|Casting|CastToPlayerController (Components|GetOwner)))
  (Variables|Default|SetAs플레이어%20컨트롤러 _as플레이어_컨트롤러_2))