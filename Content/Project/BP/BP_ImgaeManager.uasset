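; Image manager actor that shows saved high-resolution screenshots in a widget's image slots.
; On BeginPlay it finds HighresScreenshot PNGs in the screenshot folder, sorts the names descending and imports each as a Texture2D.
; It assigns the textures by index to the Image children of the widget's WrapBox, then clears the texture array.
; The code that creates the widget and adds it to the viewport is disconnected and never runs.
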(event EventBeginPlay
  (bind _returnvalue (Class|CaptureFunctionLibrary|GetPNGsOFPath (Class|BlueprintPathsLibrary|ScreenShotDir) "HighresScreenshot*.png"))
  (bind _returnvalue_2 (Class|ArrayHelperBPLibrary|SortString _returnvalue false))
  (bind _output_get (Variables|Default|SetPNGsPath _returnvalue_2))
  (for _array_element _output_get
    (bind _returnvalue_3 (Class|KismetRenderingLibrary|ImportFileasTexture2D (Utilities|String|Append (Class|BlueprintPathsLibrary|ScreenShotDir) _array_element)))
    (Utilities|Array|Add (Variables|Default|GetPNGsPath%20Import%20Texture2D) _returnvalue_3))
  (for (_array_element_2 _array_index) (Variables|Default|GetPNGsPath%20Import%20Texture2D)
    (bind _as이미지 (Utilities|Casting|CastToImage (Utilities|Array|Get(acopy) (Class|PanelWidget|GetAllChildren (Variables|/Game/Project/BP/NewWidgetBlueprint.NewWidgetBlueprint_C|GetWrapBox_73 (Variables|Default|GetWidget))) _array_index)))
    (Appearance|SetBrushfromTexture _as이미지 _array_element_2 false))
  (Utilities|Array|Clear (Variables|Default|GetPNGsPath%20Import%20Texture2D)))

(event Collision|EventActorBeginOverlap
  (params (OtherActor :type Actor%20Object%20Reference)))

(event EventTick
  (params (DeltaSeconds :type Float%20%28single-precision%29)))

(fn ConstructionScript)