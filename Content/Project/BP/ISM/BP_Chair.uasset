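; BP_Chair is a placeable actor that builds a row of chair pieces from instanced static meshes.
; Its construction script adds SpawnCount instances along local X, spaced by SpawnPosition.X and starting one step from the origin.
; A second instanced mesh adds one X-mirrored piece at the last position, apparently as an end cap.
; SpawnPosition.Y is multiplied by zero, so it has no effect, and the event graph is empty.
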(event EventBeginPlay)

(event Collision|EventActorBeginOverlap
  (params (OtherActor :type Actor%20Object%20Reference)))

(event EventTick
  (params (DeltaSeconds :type Float%20%28single-precision%29)))

(fn ConstructionScript
  (bind _spawnposition (Variables|Default|GetSpawnPosition))
  (bind _spawnposition_2 (Variables|Default|GetSpawnPosition))
  (Utilities|FlowControl|Sequence
    (:then_0
      (for _index (range 1 (Variables|Default|GetSpawnCount))
        (Components|InstancedStaticMesh|AddInstance (Variables|Default|GetInstancedStaticMesh) (Math|Transform|MakeTransform (+ (* (Math|Vector|MakeVector 0.0 0.0 0.0) (Math|Vector|MakeVector 0.0 (.y _spawnposition_2) 0.0)) (Math|Vector|MakeVector (* (.x _spawnposition_2) _index) 0.0 0.0)) "0, 0, 0" "1.000000,1.000000,1.000000") false)))
    (:then_1
      (Components|InstancedStaticMesh|AddInstance (Variables|Default|GetInstancedStaticMesh1) (Math|Transform|MakeTransform (+ (* (Math|Vector|MakeVector 0.0 0.0 0.0) (Math|Vector|MakeVector 0.0 (.y _spawnposition) 0.0)) (Math|Vector|MakeVector (* (.x _spawnposition) (Variables|Default|GetSpawnCount)) 0.0 0.0)) "0, 0, 0" "-1.000000,1.000000,1.000000") false))))