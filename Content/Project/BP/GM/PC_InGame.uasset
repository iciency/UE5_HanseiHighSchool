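; In-game player controller that owns the settings menu and toggles it with the O key.
; On BeginPlay it creates the BP_Setting widget hidden, adds it to the viewport, hides its exit panel, then runs its default and init setup.
; OpenSetting uses two parallel FlipFlops: one tracks IsOpenSetting, the other switches widget visibility, input mode, cursor, click events and game pause.
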(event Custom|OpenSetting
  (bind _returnvalue (Game|GetPlayerController 0))
  (bind _bp_setting (Variables|Default|GetBP_Setting))
  (Utilities|FlowControl|Sequence
    (:then_0
      (Utilities|FlowControl|FlipFlop
        (:A
          (Variables|Default|SetIsOpenSetting true))
        (:B
          (Variables|Default|SetIsOpenSetting false))))
    (:then_1
      (Utilities|FlowControl|FlipFlop
        (:A
          (Widget|SetVisibility _bp_setting "SelfHitTestInvisible")
          (Input|SetInputModeGameandUI _returnvalue 0 "DoNotLock" false false)
          (Variables|Default|SetbShowMouseCursor true)
          (Variables|Default|SetbEnableClickEvents true)
          (Game|SetGamePaused true))
        (:B
          (Widget|SetVisibility _bp_setting "Hidden")
          (Input|SetInputModeGameOnly _returnvalue false)
          (Variables|Default|SetbShowMouseCursor false)
          (Variables|Default|SetbEnableClickEvents false)
          (Game|SetGamePaused false))))))

(event EventBeginPlay
  (Utilities|FlowControl|Sequence
    (:then_0
      (bind _returnvalue (UserInterface|CreateWidget "/Game/Project/BP/Widget/BP_Setting.BP_Setting_C" (Game|GetPlayerController 0)))
      (Widget|SetVisibility _returnvalue "Hidden")
      (UserInterface|Viewport|AddtoViewport _returnvalue 0)
      (Variables|Default|SetBP_Setting _returnvalue)
      (Widget|SetVisibility (Variables|/Game/Project/BP/Widget/BP_Setting.BP_Setting_C|GetExitPanel _returnvalue) "Hidden"))
    (:then_1
      (Default|DefualtSetting (Variables|Default|GetBP_Setting))
      (Default|InitSetting (Variables|Default|GetBP_Setting)))))

(event EventTick
  (params (DeltaSeconds :type Float%20%28single-precision%29)))

(event Input|KeyboardEvents|O
  (params (Key :type Key%20Structure :default "None"))
  (:Pressed
    (CallFunction|OpenSetting)))

(fn ConstructionScript)