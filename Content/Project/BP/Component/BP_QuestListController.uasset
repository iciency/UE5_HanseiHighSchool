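; BP_QuestListController handles keyboard control of the quest list widget, the UI that shows captured images.
; On BeginPlay it finds BP_ImageManager in the level, takes its QuestListWidget, and adds that to the viewport hidden.
; V toggles visibility through a FlipFlop.
; While the widget is not hidden, C and B call its UpdateImage with opposite boolean arguments.
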(event EventBeginPlay
  (Utilities|FlowControl|Sequence
    (:then_0
      (bind _returnvalue (Actor|GetActorOfClass "/Game/Project/BP/BP_ImageManager.BP_ImageManager_C"))
      (Variables|Default|SetBP_ImageManager _returnvalue))
    (:then_1
      (UserInterface|Viewport|AddtoViewport (Variables|/Game/Project/BP/BP_ImageManager.BP_ImageManager_C|GetQuestListWidget (Variables|Default|GetBP_ImageManager)) 0)
      (Widget|SetVisibility (Variables|/Game/Project/BP/BP_ImageManager.BP_ImageManager_C|GetQuestListWidget (Variables|Default|GetBP_ImageManager)) "Hidden"))))

(event Input|KeyboardEvents|B
  (params (Key :type Key%20Structure :default "None"))
  ;[1 1 1] 켑쳐한 이미지의 UI 보여주는 놈
  (:Pressed
    (if (not (Utilities|Enum|Equal(Enum) (Widget|GetVisibility (Variables|/Game/Project/BP/BP_ImageManager.BP_ImageManager_C|GetQuestListWidget (Variables|Default|GetBP_ImageManager))) "Hidden"))
      (Default|UpdateImage (Variables|/Game/Project/BP/BP_ImageManager.BP_ImageManager_C|GetQuestListWidget (Variables|Default|GetBP_ImageManager)) false))))

(event Input|KeyboardEvents|V
  (params (Key :type Key%20Structure :default "None"))
  (bind _bp_imagemanager (Variables|Default|GetBP_ImageManager))
  (bind _questlistwidget (Variables|/Game/Project/BP/BP_ImageManager.BP_ImageManager_C|GetQuestListWidget _bp_imagemanager))
  ;[1 1 1] 켑쳐한 이미지의 UI 보여주는 놈
  (:Pressed
    (Utilities|FlowControl|FlipFlop
      (:A
        (Widget|SetVisibility _questlistwidget "Visible"))
      (:B
        (Widget|SetVisibility _questlistwidget "Hidden")))))

(event Input|KeyboardEvents|C
  (params (Key :type Key%20Structure :default "None"))
  ;[1 1 1] 켑쳐한 이미지의 UI 보여주는 놈
  (:Pressed
    (if (not (Utilities|Enum|Equal(Enum) (Widget|GetVisibility (Variables|/Game/Project/BP/BP_ImageManager.BP_ImageManager_C|GetQuestListWidget (Variables|Default|GetBP_ImageManager))) "Hidden"))
      (Default|UpdateImage (Variables|/Game/Project/BP/BP_ImageManager.BP_ImageManager_C|GetQuestListWidget (Variables|Default|GetBP_ImageManager)) true))))